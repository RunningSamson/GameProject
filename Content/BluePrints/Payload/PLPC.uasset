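; Player controller for the Payload mode that handles team and character selection, spawning, death and respawn, and session exit.
; Initial setup caches game mode and player state, loads saved player settings, and creates the team-choice widget and hidden hold-to-show scoreboard.
; Assigning a character saves it, refreshes all scoreboards through PLGM, and possesses a pawn spawned at a random team start.
; Death records the stat, then respawns after a delay.
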(event `Initial Setup`
  ;[1 1 1] Initial Setup
  (`self.ChooseTeamWidget`)
  (`self.Create PlayerOverview`)
  (bind _asplgm (cast `/Game/BluePrints/Payload/PLGM` (`GameplayStatics.GetGameMode`)))
  (set `self.PLGMREF` _asplgm)
  (bind _asplps (cast `/Game/BluePrints/Payload/PLPS` (`self.PlayerState`)))
  (set `self.PLPSREF` _asplps))

(event `ChooseTeamWidget`
  ;[0.001347 0 1] Widgets
  ;;[1 1 1] Choose Team Widget
  (`self.Check Save Game`)
  (bind _returnvalue (`|CreateWidget` "/Game/Game/UI/Test/ChooseTeam.ChooseTeam_C"))
  (`UserWidget.AddToViewport` _returnvalue 0)
  (`WidgetBlueprintLibrary.SetInputMode_GameAndUIEx` self null))

(event `ChooseCharacterWidget`
  ;[0.001347 0 1] Widgets
  ;;[1 1 1] Choose Character Widget
  (bind _returnvalue (`|CreateWidget` "/Game/Game/UI/Test/ChooseCharacter.ChooseCharacter_C"))
  (`UserWidget.AddToViewport` _returnvalue 0))

(event `Create PlayerOverview`
  ;[0.001347 0 1] Widgets
  ;;[1 1 1] Scoreboard
  ;;;[1 1 1] Create Scoreboard
  (bind _returnvalue (`|CreateWidget` "/Game/Game/UI/Test/PlayerOverview.PlayerOverview_C"))
  (bind _output_get (set `self.PlayerOverviewREF` _returnvalue))
  (`UserWidget.AddToViewport` _output_get 0)
  (`Widget.SetVisibility` _output_get "Hidden"))

(event `InputAction|PlayerOverview`
  (params (Key :type "Key Structure"))
  (bind _playeroverviewref (`self.PlayerOverviewREF`))
  ;[0.001347 0 1] Widgets
  ;;[1 1 1] Scoreboard
  ;;;[1 1 1] Show / Hide Scoreboard
  (:`Pressed`
    (`Widget.SetVisibility` _playeroverviewref "Visible"))
  (:`Released`
    (`Widget.SetVisibility` _playeroverviewref "Hidden")))

(event `Add Player Info`
  (params (`Connected Players` :type "Array of /Game/BluePrints/AllLevels/PlayerInfo Structure") (PLPS :type "Array of PlayerState Object Reference"))
  (bind _playeroverviewref (`self.PlayerOverviewREF`))
  ;[0.001347 0 1] Widgets
  ;;[1 1 1] Scoreboard
  ;;;[1 1 1] Add player info to scoreboard
  (set `self.Connected Players` `Connected Players`)
  (set `self.PLPS` PLPS)
  (`/Engine/EditorBlueprintResources/StandardMacros.IsValid` _playeroverviewref
    (:`Is Valid`
      (`/Game/Game/UI/Test/PlayerOverview.Clear Player Window` _playeroverviewref)
      (for (_array_element _array_index) (`self.Connected Players`)
        (`/Game/Game/UI/Test/PlayerOverview.Update Player Window` _playeroverviewref _array_element (`|GetArrayItem` (`self.PLPS`) _array_index))))))

(event `Call Update`
  (params (`Player Info` :type "/Game/BluePrints/AllLevels/PlayerInfo Structure"))
  ;[0.001347 0 1] Widgets
  ;;[1 1 1] Scoreboard
  ;;;[1 1 1] Update all players' scoreboard
  (set `self.PlayerSettings` `Player Info`)
  (bind _asplgm (cast `/Game/BluePrints/Payload/PLGM` (`GameplayStatics.GetGameMode`)))
  (`/Game/BluePrints/Payload/PLGM.All Update` _asplgm))

(event `Assign Character`
  (params (Character :type "Character Class Reference"))
  ;[1 1 1] Assign Character
  (setmembers `/Game/BluePrints/AllLevels/PlayerInfo` :`StructRef` (`self.PlayerSettings`) :`MyPlayerCharacter` Character)
  (set `self.PlayerCharacterREF` Character)
  (`self.SaveGame`)
  (`self.Call Update` (`self.PlayerSettings`))
  (`WidgetBlueprintLibrary.SetInputMode_GameOnly` self)
  (`self.Respawn`))

(event `Respawn`
  (bind (_myplayername _myplayerimg _myplayercharacter _myplayercharacterimg _myplayerstatus _myteamname) (break `/Game/BluePrints/AllLevels/PlayerInfo` (`self.PlayerSettings`)))
  (bind _playerstart_teama (`/Game/BluePrints/Payload/PLGM.PlayerStart TeamA` (`self.PLGMREF`)))
  (bind _playerstart_teamb (`/Game/BluePrints/Payload/PLGM.PlayerStart TeamB` (`self.PLGMREF`)))
  ;[1 0 0] Respawn
  (`/Engine/EditorBlueprintResources/StandardMacros.IsValid` (`self.K2_GetPawn`)
    (:`Is Valid`
      (`self.K2_DestroyActor`))
    (:`Is Not Valid`
      _))
  (if (`KismetStringLibrary.EqualEqual_StrStr` (`KismetTextLibrary.Conv_TextToString` _myteamname) "TeamA")
    (bind _returnvalue (`|SpawnActorFromClass` _myplayercharacter (`self.GetTransform` (`|GetArrayItem` _playerstart_teama (`KismetMathLibrary.RandomIntegerInRange` 0 (- (`KismetArrayLibrary.Array_Length` _playerstart_teama) 1)))) "Undefined" "OverrideRootScale" null null))
    (`self.Possess` _returnvalue)
    (else
      (bind _returnvalue_2 (`|SpawnActorFromClass` _myplayercharacter (`self.GetTransform` (`|GetArrayItem` _playerstart_teamb (`KismetMathLibrary.RandomIntegerInRange` 0 (- (`KismetArrayLibrary.Array_Length` _playerstart_teamb) 1)))) "Undefined" "OverrideRootScale" null null))
      (`self.Possess` _returnvalue_2)))
  (set `self.ReadyToStart?` true))

(event `self.ReceiveUnPossess`
  (params (UnpossessedPawn :type "Pawn Object Reference"))
  (bind _controlled_pawn (`self.Controlled Pawn`))
  ;[1 0 0] Respawn
  ;;[1 1 1] When Unpossesd Respawn
  (`/Engine/EditorBlueprintResources/ActorMacros.Switch Has Authority`
    (:`Authority`
      (`/Engine/EditorBlueprintResources/StandardMacros.IsValid` _controlled_pawn
        (:`Is Valid`
          (`self.K2_DestroyActor` _controlled_pawn))
        (:`Is Not Valid`
          _))
      (`KismetSystemLibrary.Delay` (`self.Respawn Delay`))
      (`self.Respawn`))))

(event `OnDeath`
  ;[1 0 0] Respawn
  ;;[1 1 1] Player Has Died
  (set `self.Controlled Pawn` (`self.K2_GetPawn` self))
  (`self.UnPossess`)
  (`/Game/BluePrints/Payload/PLPS.Add Death` (`self.PLPSREF`))
  (`/Game/BluePrints/Payload/PLGM.All Update` (`self.PLGMREF`))
  (`KismetSystemLibrary.Delay` (`self.Respawn Delay`))
  (`GameModeBase.RestartPlayer` (`GameplayStatics.GetGameMode`) null))

(event `Show Countdown`
  ;[1 1 1] Show Countdown
  (bind _returnvalue (`|CreateWidget` "/Game/Game/UI/Test/Countdown.Countdown_C"))
  (`UserWidget.AddToViewport` _returnvalue 0))

(event `Key|Escape`
  (params (Key :type "Key Structure"))
  ;[1 1 1] Destroy with esc
  (:`Pressed`
    (`DestroySessionCallbackProxy.DestroySession` self
      (:`OnSuccess`
        (`GameplayStatics.OpenLevel` "MainMenu")))))

(fn `Check Save Game`
  (bind _returnvalue (`GameplayStatics.DoesSaveGameExist` (`self.PlayerSettingsSave`)))
  (if _returnvalue
    (`self.LoadGame`)
    (`self.SaveGame`)
    (else
      (`self.SaveGame`))))

(fn `LoadGame`
  (bind _returnvalue (`GameplayStatics.LoadGameFromSlot` (`self.PlayerSettingsSave`)))
  (bind _asplayer_save_game (cast `/Game/BluePrints/AllLevels/PlayerSaveGame` _returnvalue))
  (bind (_myplayername _myplayerimg _myplayercharacter) (break `/Game/BluePrints/AllLevels/PlayerInfo` (`/Game/BluePrints/AllLevels/PlayerSaveGame.S_PlayerInfo` _asplayer_save_game)))
  (setmembers `/Game/BluePrints/AllLevels/PlayerInfo` :`StructRef` (`self.PlayerSettings`) :`MyPlayerName` _myplayername :`MyPlayerImg` _myplayerimg :`MyPlayerCharacter` "/Game/BluePrints/Characters/Rian/Rian.Rian_C" :`MyPlayerCharacterImg` null :`MyPlayerStatus` "NotReady")
  (set `self.PlayerCharacterREF` _myplayercharacter))

(fn `SaveGame`
  (`/Engine/EditorBlueprintResources/StandardMacros.IsValid` (`self.PlayerSaveGameREF`)
    (:`Is Valid`
      _)
    (:`Is Not Valid`
      (bind _returnvalue (`GameplayStatics.CreateSaveGameObject` "/Game/BluePrints/AllLevels/PlayerSaveGame.PlayerSaveGame_C"))
      (bind _asplayer_save_game (cast `/Game/BluePrints/AllLevels/PlayerSaveGame` _returnvalue))
      (set `self.PlayerSaveGameREF` _asplayer_save_game)))
  (set `/Game/BluePrints/AllLevels/PlayerSaveGame.S_PlayerInfo` (`self.PlayerSettings`) (`self.PlayerSaveGameREF`))
  (`GameplayStatics.SaveGameToSlot` null (`self.PlayerSettingsSave`)))

(fn `UserConstructionScript`)