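; Player controller for the Payload game mode that handles input mode and the countdown UI.
; BeginPlay switches input to game-only, then casts to PayloadGM and loops over all Pawns with an empty loop body.
; The ShowCountdown event creates a Countdown widget owned by this controller and adds it to the viewport.
; An unconnected scoreboard widget branch has no class set and never runs.
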(event `self.ReceiveBeginPlay`
  (`WidgetBlueprintLibrary.SetInputMode_GameOnly` self)
  (cast `/Game/BluePrints/Payload/PayloadGM` (`GameplayStatics.GetGameMode`))
  (bind _outactors (`GameplayStatics.GetAllActorsOfClass` "/Script/Engine.Pawn"))
  (for _ _outactors
    _))

(event `Show Countdown`
  ;[1 1 1] Show Countdown
  (bind _returnvalue (`|CreateWidget` "/Game/Game/UI/Payload/Countdown.Countdown_C" self))
  (`UserWidget.AddToViewport` _returnvalue 0))

(fn `UserConstructionScript`)