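; Payload game mode that gathers joining players, runs a match timer and handles spawning and respawning.
; PostLogin shows each PayloadPC's countdown once the lobby fills, and BeginPlay caches Red and Blue tagged PlayerStarts.
; A Delay on Tick drives the timer; on expiry, SpawnPlayers creates local players possessing Rian pawns, looping only over Red starts.
; OnPlayerKilled unpossesses and restarts the player, while KillPlayer is an empty stub.
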(event `self.K2_PostLogin`
  (params (NewPlayer :type "PlayerController Object Reference"))
  ;[1 1 1] Player Count + Start Countdown When max is reached
  (bind _aspayload_pc (cast `/Game/BluePrints/Payload/PayloadPC` NewPlayer))
  (`KismetArrayLibrary.Array_Add` (`self.Players`) _aspayload_pc)
  (if (== (`KismetArrayLibrary.Array_Length` (`self.Players`)) (`self.MaxPlayerCountTotal`))
    (`KismetSystemLibrary.Delay` 2.0)
    (for _array_element (`self.Players`)
      (`/Game/BluePrints/Payload/PayloadPC.Show Countdown` _array_element)
      (`WidgetBlueprintLibrary.SetInputMode_GameOnly` NewPlayer))))

(event `self.ReceiveBeginPlay`
  (`WidgetBlueprintLibrary.SetInputMode_GameOnly` (`GameplayStatics.GetPlayerController` 0))
  (bind _outactors (`GameplayStatics.GetAllActorsOfClassWithTag` "/Script/Engine.PlayerStart" "Red"))
  (`KismetArrayLibrary.Array_Clear` (`self.RedTeamStart`))
  (set `self.RedTeamStart` _outactors)
  (bind _outactors_2 (`GameplayStatics.GetAllActorsOfClassWithTag` "/Script/Engine.PlayerStart" "Blue"))
  (`KismetArrayLibrary.Array_Clear` (`self.BlueTeamStart`))
  (set `self.BlueTeamStart` _outactors_2))

(event `self.ReceiveTick`
  (params (DeltaSeconds :type "Float (single-precision)"))
  (`KismetSystemLibrary.Delay` 1.0)
  (set `self.Seconds` (- (`self.Seconds`) 1))
  (if (< (`self.Seconds`) 0)
    (set `self.Minutes` (- (`self.Minutes`) 1))
    (set `self.Seconds` 59)
    (if (<= (`self.Minutes`) -1)
      (`KismetSystemLibrary.PrintString` "Time's up")
      (`self.Get Player Start Points`)
      (`self.SpawnPlayers`))))

(event `Countdown`
  ;[1 1 1] Show Countdown
  (for _array_element (`self.Players`)
    (`/Game/BluePrints/Payload/PayloadPC.Show Countdown` _array_element)))

(fn `Get Player Start Points`
  (bind _outactors (`GameplayStatics.GetAllActorsOfClassWithTag` "/Script/Engine.PlayerStart" "Red"))
  (set `self.RedTeamStart` _outactors)
  (bind _outactors_2 (`GameplayStatics.GetAllActorsOfClassWithTag` "/Script/Engine.PlayerStart" "Blue"))
  (set `self.BlueTeamStart` _outactors_2))

(fn `KillPlayer`)

(fn `OnPlayerKilled`
  (params (Player :type "Character Object Reference"))
  (locals (PlayerController :type "Controller Object Reference"))
  (bind _output_get (set `local.PlayerController` (`Pawn.GetController` Player)))
  (`Controller.UnPossess` _output_get)
  (`self.RestartPlayer` (`local.PlayerController`)))

(fn `SpawnPlayers`
  (bind _index (`self.Index`))
  (bind _index_2 (`self.Index`))
  (for _index_3 (range (`self.MaxPlayerCountInTeam`))
    (set `self.Index` _index_3)
    (for _array_element (`self.RedTeamStart`)
      (if (== (`PlayerStart.PlayerStartTag` _array_element) (`KismetStringLibrary.Conv_StringToName` (`KismetStringLibrary.Conv_IntToString` (`self.Index`))))
        (`GameplayStatics.CreatePlayer` _index_2)
        (bind _returnvalue (`|SpawnActorFromClass` "/Game/Characters/Rian.Rian_C" (`self.GetTransform` _array_element) "AlwaysSpawn" "OverrideRootScale" null null))
        (`Controller.Possess` (`GameplayStatics.GetPlayerController` _index_2) _returnvalue)
        (else
          (`GameplayStatics.CreatePlayer` _index)
          (bind _returnvalue_2 (`|SpawnActorFromClass` "/Game/Characters/Rian.Rian_C" (`self.GetTransform` _array_element) "AlwaysSpawn" "OverrideRootScale" null null))
          (`Controller.Possess` (`GameplayStatics.GetPlayerController` _index) _returnvalue_2))))))

(fn `UserConstructionScript`)