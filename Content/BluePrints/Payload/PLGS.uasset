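; Game State for the Payload mode that gates match start and runs the round clock.
; On authority it caches the PLGM game mode and player limit; CanStart? checks controller pawns once full, then shows the countdown or retries after a delay.
; A looping timer event decrements Minutes and Seconds, calling the game mode's RoundHasEnded when Minutes decrements to zero.
; Other round events are empty stubs.
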(event `self.ReceiveBeginPlay`
  ;[1 1 1] Get Max Players
  (`/Engine/EditorBlueprintResources/ActorMacros.Switch Has Authority`
    (:`Authority`
      (bind _asplgm (cast `/Game/BluePrints/Payload/PLGM` (`GameplayStatics.GetGameMode`)))
      (set `self.PLGM REF` _asplgm)
      (set `self.Max Players` (`/Game/BluePrints/Payload/PLGM.Max Players` _asplgm)))))

(event `CanStart?`
  (params (`Current Players` :type Integer))
  (bind _plgm_ref (`self.PLGM REF`))
  ;[1 1 1] Check If Players Have Pawns + Start Match
  (bind _output_get (set `self.Current Players` `Current Players`))
  (if (== _output_get (`self.Max Players`))
    (for _array_element (`/Game/BluePrints/Payload/PLGM.AllPlayerControllers` _plgm_ref)
      (bind _asplpc (cast `/Game/BluePrints/Payload/PLPC` _array_element))
      (`/Engine/EditorBlueprintResources/StandardMacros.IsValid` (`Controller.K2_GetPawn` _asplpc)
        (:`Is Valid`
          (set `self.GameCanStart?` true))
        (:`Is Not Valid`
          (set `self.GameCanStart?` false))))
    (if (`self.GameCanStart?`)
      (`/Game/BluePrints/Payload/PLGM.Show Countdown` _plgm_ref)
      (else
        (`KismetSystemLibrary.PrintString` "Not Ready to start!")
        (`KismetSystemLibrary.Delay` 1.0)
        (`self.CanStart?` (`self.Current Players`))))))

(event `SR OnStartOfRound`
  (set `self.Minutes` 5)
  (set `self.Seconds` 0)
  (`KismetSystemLibrary.K2_SetTimerDelegate` (delegate `SR Update Timer`) 1.0 true))

(event `SR Update Timer`
  (`self.Timer`))

(event `SR OnRoundHasEnded`)

(event `New Round Started`)

(event `/Game/BluePrints/Payload/BPI_StartGame.StartGame`)

(fn `UserConstructionScript`)