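; Payload actor that travels along a track spline while its sphere trigger is overlapped, stopping on end overlap.
; A timeline, rate-scaled by Duration and started at an offset, drives Alpha, which BeginLocation maps to spline distance to set location and rotation.
; When the timeline finishes, it respawns every player through the PayloadGM game mode, resets the match timer and rewinds the timeline.
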(event `self.Sphere.OnComponentBeginOverlap`
  (params (OverlappedComponent :type "PrimitiveComponent Object Reference") (OtherActor :type "Actor Object Reference") (OtherComp :type "PrimitiveComponent Object Reference") (OtherBodyIndex :type Integer) (bFromSweep :type Boolean) (SweepResult :type "HitResult Structure (by ref)"))
  (set `self.ActivePayload` true)
  (if (`self.ActivePayload`)
    (`self.MovePayload`)))

(event `MovePayload`
  (bind _payloadgmref (`self.PayloadGMREF`))
  (bind (_direction _alpha) (`Timeline|PayloadMover` :!label _label)
    (:`Update`
      (set `self.Alpha` _alpha)
      (`self.BeginLocation`))
    (:`Finished`
      ;[1 1 1] Respawn Players + reset timer
      (bind _aspayload_gm (cast `/Game/BluePrints/Payload/PayloadGM` (`GameplayStatics.GetGameMode`)))
      (set `self.PayloadGMREF` _aspayload_gm)
      (for _array_element (`/Game/BluePrints/Payload/PayloadGM.Players` _aspayload_gm)
        (`/Game/BluePrints/Payload/PayloadGM.Respawn Player` (`self.PayloadGMREF`) _array_element (`.MyPlayerCharacter_9_9E65376B496BA5B65D4476B1B5EF252E` (break `/Game/BluePrints/AllLevels/PlayerInfo` (`/Game/BluePrints/Payload/PayloadPC.Player Settings` _array_element)))))
      (set `/Game/BluePrints/Payload/PayloadGM.Minutes` 6 _payloadgmref)
      (set `/Game/BluePrints/Payload/PayloadGM.Seconds` 0 _payloadgmref)
      (`TimelineComponent.SetNewTime` (`self.PayloadMover`) 0.0)
      (goto _label :!via `SetNewTime`))))

(event `self.ReceiveBeginPlay`
  (`TimelineComponent.SetPlayRate` (`self.PayloadMover`) (/ 1.0 (`self.Duration`)))
  (`TimelineComponent.SetNewTime` (`self.PayloadMover`) (`self.PayloadStartOffset`))
  (goto _label :!via `SetNewTime`))

(event `StopPayload`
  (goto _label :!via `Stop`))

(event `self.Sphere.OnComponentEndOverlap`
  (params (OverlappedComponent :type "PrimitiveComponent Object Reference") (OtherActor :type "Actor Object Reference") (OtherComp :type "PrimitiveComponent Object Reference") (OtherBodyIndex :type Integer))
  (set `self.ActivePayload` false)
  (set `self.Alpha` 0.0)
  (goto _label :!via `Stop`))

(fn `BeginLocation`
  (bind _returnvalue (`KismetMathLibrary.Lerp` 0.0 (`SplineComponent.GetSplineLength` (`/Game/BluePrints/Payload/Track.PayloadSpline` (`self.TrackRef`))) (`self.Alpha`)))
  (`self.K2_SetActorLocationAndRotation` (`SplineComponent.GetLocationAtDistanceAlongSpline` (`/Game/BluePrints/Payload/Track.PayloadSpline` (`self.TrackRef`)) _returnvalue "World") (`SplineComponent.GetRotationAtDistanceAlongSpline` (`/Game/BluePrints/Payload/Track.PayloadSpline` (`self.TrackRef`)) _returnvalue "World")))

(fn `UserConstructionScript`)