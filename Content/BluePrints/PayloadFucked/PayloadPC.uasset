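; PayloadPC is the player controller for the payload game mode, handling setup, countdown display and exiting to the main menu.
; On BeginPlay the local controller clears widgets, loads saved player settings and passes them to PassCharacterInfoToServer, which has PayloadGM respawn the player as the chosen character.
; ShowCountdown adds a countdown widget for the local player.
; Escape opens MainMenu and destroys the session.
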(event `self.ReceiveBeginPlay`
  ;[1 1 1] Begin play
  (`WidgetBlueprintLibrary.SetInputMode_GameOnly` self)
  (if (`self.IsLocalController`)
    (`WidgetLayoutLibrary.RemoveAllWidgets`)
    (`self.Load Game`)
    (`self.PassCharacterInfoToServer` (`self.Player Settings`))))

(event `PassCharacterInfoToServer`
  (params (PlayerSettingsInfo :type "/Game/BluePrints/AllLevels/PlayerInfo Structure"))
  ;[1 1 1] Pass Character info
  (set `self.Player Settings` PlayerSettingsInfo)
  (bind _aspayload_gm (cast `/Game/BluePrints/PayloadFucked/PayloadGM` (`GameplayStatics.GetGameMode`)))
  (`/Game/BluePrints/PayloadFucked/PayloadGM.Respawn Player` _aspayload_gm self (`.MyPlayerCharacter_9_9E65376B496BA5B65D4476B1B5EF252E` (break `/Game/BluePrints/AllLevels/PlayerInfo` (`self.Player Settings`)))))

(event `Show Countdown`
  ;[1 1 1] Show Countdown
  (if (`self.IsLocalController`)
    (bind _returnvalue (`|CreateWidget` "/Game/Game/UI/Test/Countdown.Countdown_C" self))
    (`UserWidget.AddToViewport` _returnvalue 0)
    (`KismetSystemLibrary.PrintString` "Show")))

(event `Key|Escape`
  (params (Key :type "Key Structure"))
  ;[1 1 1] Destroy with esc
  (:`Pressed`
    (`GameplayStatics.OpenLevel` "MainMenu")
    (`DestroySessionCallbackProxy.DestroySession` self)))

(fn `Load Game`
  (bind _returnvalue (`GameplayStatics.LoadGameFromSlot` (`self.PlayerSettingsSave`)))
  (bind _asplayer_save_game (cast `/Game/BluePrints/AllLevels/PlayerSaveGame` _returnvalue))
  (set `self.Player Settings` (`/Game/BluePrints/AllLevels/PlayerSaveGame.S_PlayerInfo` _asplayer_save_game)))

(fn `UserConstructionScript`)