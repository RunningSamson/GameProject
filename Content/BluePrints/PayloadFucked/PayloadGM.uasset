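; Game mode for a two-team Payload match that gathers players, spawns them by team and handles logouts.
; On controller swap it carries tags over and, once GameInfoInstance's MaxPlayers is reached, shows each player a countdown after a delay.
; RespawnPlayer spawns and possesses a Rian at a random Red or Blue PlayerStart chosen by controller tag.
; ReadyToStartMatch always returns false, and logout calls the game instance's session teardown.
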(event `self.ReceiveBeginPlay`)

(event `self.K2_OnSwapPlayerControllers`
  (params (OldPC :type "PlayerController Object Reference") (NewPC :type "PlayerController Object Reference"))
  (set `Actor.Tags` (`Actor.Tags` OldPC) NewPC)
  (`KismetArrayLibrary.Array_Add` (`self.AllPlayerControllers`) NewPC)
  ;[1 1 1] Player Controller Swap + starting countdown if max players
  (bind _returnvalue (`self.GetNumPlayers`))
  (`KismetSystemLibrary.PrintString` (`KismetStringLibrary.Conv_IntToString` _returnvalue))
  (bind _returnvalue_2 (`self.Getting Max Players` NewPC))
  (if _returnvalue_2
    (`KismetSystemLibrary.Delay` 3.0)
    (for _array_element (`self.Players`)
      (`/Game/BluePrints/PayloadFucked/PayloadPC.Show Countdown` _array_element))
    (else
      (`KismetSystemLibrary.PrintString` "Not Enough Players"))))

(event `Respawn All Players`
  ;[1 1 1] Respawn All Players
  (bind _outactors (`GameplayStatics.GetAllActorsOfClass` "/Script/Engine.Character"))
  (for _array_element _outactors
    (`self.OnPlayerKilled` _array_element)))

(event `Respawn Player`
  (params (`Player Controller` :type "PlayerController Object Reference") (`Player Character` :type "Character Class Reference"))
  (bind _returnvalue (`Controller.K2_GetPawn` `Player Controller`))
  (bind _redteamspawnpoint (`self.RedTeamSpawnPoint`))
  (bind _blueteamspawnpoint (`self.BlueTeamSpawnpoint`))
  ;[1 1 1] Spawn Player with Character
  (`self.Get Player Start Points`)
  (`/Engine/EditorBlueprintResources/StandardMacros.IsValid` _returnvalue
    (:`Is Valid`
      (`self.K2_DestroyActor` _returnvalue))
    (:`Is Not Valid`
      _))
  (if (`KismetArrayLibrary.Array_Contains` (`Actor.Tags` `Player Controller`) "Red")
    (bind _returnvalue_2 (`|SpawnActorFromClass` "/Game/BluePrints/Characters/Rian/Rian.Rian_C" (`self.GetTransform` (`|GetArrayItem` _redteamspawnpoint (`KismetMathLibrary.RandomIntegerInRange` 0 (- (`KismetArrayLibrary.Array_Length` _redteamspawnpoint) 1)))) "Undefined" "OverrideRootScale" null 1000 null))
    (`Controller.Possess` `Player Controller` _returnvalue_2)
    (else
      (bind _returnvalue_3 (`|SpawnActorFromClass` "/Game/BluePrints/Characters/Rian/Rian.Rian_C" (`self.GetTransform` (`|GetArrayItem` _blueteamspawnpoint (`KismetMathLibrary.RandomIntegerInRange` 0 (- (`KismetArrayLibrary.Array_Length` _blueteamspawnpoint) 1)))) "Undefined" "OverrideRootScale" null 1000 null))
      (`Controller.Possess` `Player Controller` _returnvalue_3))))

(event `self.K2_OnLogout`
  (params (ExitingController :type "Controller Object Reference"))
  ;[1 1 1] Event On logout: Destroy Session + game info instance
  (bind _aspayload_pc (cast `/Game/BluePrints/PayloadFucked/PayloadPC` ExitingController))
  (`/Game/BluePrints/AllLevels/GameInfoInstance.Destroy Session Caller` (cast `/Game/BluePrints/AllLevels/GameInfoInstance` (`GameplayStatics.GetGameInstance`) :!pure true) _aspayload_pc))

(event `self.ReceiveTick`
  (params (DeltaSeconds :type "Float (single-precision)")))

(fn `Get Player Start Points`
  (bind _outactors (`GameplayStatics.GetAllActorsOfClass` "/Script/Engine.PlayerStart"))
  (for _array_element _outactors
    (if (== (`PlayerStart.PlayerStartTag` _array_element) "Red")
      (`KismetArrayLibrary.Array_Add` (`self.RedTeamSpawnPoint`) _array_element)
      (else
        (`KismetArrayLibrary.Array_Add` (`self.BlueTeamSpawnpoint`) _array_element)))))

(fn `KillPlayer`)

(fn `OnPlayerKilled`
  (params (Player :type "Character Object Reference"))
  (locals (PlayerController :type "Controller Object Reference"))
  (bind _output_get (set `local.PlayerController` (`Pawn.GetController` Player)))
  (`Controller.UnPossess` _output_get)
  (`self.RestartPlayer` (`local.PlayerController`))
  (`self.K2_DestroyActor` Player))

(fn `Player Start`
  (params (`Player Controller` :type "PlayerController Object Reference"))
  (returns (`Player Start` :type "PlayerStart Object Reference"))
  (for _array_element (`Actor.Tags` `Player Controller`)
    (if (== _array_element "Red")
      (for _array_element_2 (`self.RedTeamSpawnPoint`)
        (for _array_element_3 (`Actor.Tags` _array_element_2)
          (if (== _array_element_3 "None")
            (bind _output_get (set `self.PlayerStart` _array_element_2))
            (`KismetArrayLibrary.Array_Add` (`Actor.Tags` _output_get) "Taken")
            (return (`self.PlayerStart`)))))
      (else
        (for _array_element_4 (`self.BlueTeamSpawnpoint`)
          (for _array_element_5 (`Actor.Tags` _array_element_4)
            (if (== _array_element_5 "None")
              (bind _output_get_2 (set `self.PlayerStart` _array_element_4))
              (`KismetArrayLibrary.Array_Add` (`Actor.Tags` _output_get_2) "Taken")
              (return (`self.PlayerStart`)))))))))

(fn `ReadyToStartMatch`
  (returns (ReturnValue :type Boolean))
  (return false))

(fn `UserConstructionScript`)