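; Payload game mode that assigns the player to the Random or Engineers team and spawns them as a Rian pawn.
; BeginPlay gathers tagged PlayerStarts per team, then runs team assignment and respawn.
; Assignment fills Random before Engineers, capped by start counts, opens MainMenu when both are full, and updates player info only for Random.
; Respawn picks a random team start and always possesses the pawn with player controller 0.
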(event `self.ReceiveBeginPlay`
  (bind _outactors (`GameplayStatics.GetAllActorsOfClassWithTag` "/Script/Engine.PlayerStart" "Engineers"))
  (`KismetArrayLibrary.Array_Clear` (`self.EngineersTeamStart`))
  (set `self.EngineersTeamStart` _outactors)
  (bind _outactors_2 (`GameplayStatics.GetAllActorsOfClassWithTag` "/Script/Engine.PlayerStart" "Random"))
  (`KismetArrayLibrary.Array_Clear` (`self.RandomTeamStart`))
  (set `self.RandomTeamStart` _outactors_2)
  (`self.Assign Team`)
  (`self.Respawn Player` null))

(event `Respawn Player`
  (params (PlayerControllerREF :type "PlayerController Object Reference"))
  (bind _engineersteamstart (`self.EngineersTeamStart`))
  (bind _randomteamstart (`self.RandomTeamStart`))
  (`/Engine/EditorBlueprintResources/StandardMacros.IsValid` (`Controller.K2_GetPawn` PlayerControllerREF)
    (:`Is Valid`
      (`self.K2_DestroyActor`))
    (:`Is Not Valid`
      _))
  (if (`KismetArrayLibrary.Array_Contains` (`self.PlayersEngineers`) (`.MyPlayerName_2_4AAAFA6E46CCE2F82AD6E48F8CD81397` (break `/Game/BluePrints/AllLevels/PlayerInfo` (`/Game/BluePrints/Gameplay/GameplayPC.Player Info` (`self.GamePlayControllerREF`)))))
    (bind _returnvalue (`|SpawnActorFromClass` "/Game/Characters/Rian.Rian_C" (`self.GetTransform` (`|GetArrayItem` _engineersteamstart (`KismetMathLibrary.RandomIntegerInRange` 0 (- (`KismetArrayLibrary.Array_Length` _engineersteamstart) 1)))) "Undefined" "OverrideRootScale" null null))
    (`Controller.Possess` (`GameplayStatics.GetPlayerController` 0) _returnvalue)
    (else
      (bind _returnvalue_2 (`|SpawnActorFromClass` "/Game/Characters/Rian.Rian_C" (`self.GetTransform` (`|GetArrayItem` _randomteamstart (`KismetMathLibrary.RandomIntegerInRange` 0 (- (`KismetArrayLibrary.Array_Length` _randomteamstart) 1)))) "Undefined" "OverrideRootScale" null null))
      (`Controller.Possess` (`GameplayStatics.GetPlayerController` 0) _returnvalue_2))))

(fn `Assign Team`
  (bind _myplayername (break `/Game/BluePrints/AllLevels/PlayerInfo` (`/Game/BluePrints/Gameplay/GameplayPC.Player Info` (`self.GamePlayControllerREF`))))
  (bind _aspayload_gm (cast `/Game/BluePrints/Gameplay/PayloadGM` (`GameplayStatics.GetGameMode`)))
  (if (< (`KismetArrayLibrary.Array_Length` (`/Game/BluePrints/Gameplay/PayloadGM.PlayersRandom` _aspayload_gm)) (+ (`KismetArrayLibrary.Array_Length` (`/Game/BluePrints/Gameplay/PayloadGM.RandomTeamStart` _aspayload_gm)) 1))
    (`KismetArrayLibrary.Array_Add` (`/Game/BluePrints/Gameplay/PayloadGM.PlayersRandom` _aspayload_gm) _myplayername)
    (set `self.Team Name` "Random")
    (setmembers `/Game/BluePrints/AllLevels/PlayerInfo` :`StructRef` (`/Game/BluePrints/Gameplay/GameplayPC.Player Info` (`self.GamePlayControllerREF`)) :`MyPlayerName` "" :`MyPlayerImg` null :`MyPlayerCharacter` null :`MyPlayerCharacterImg` null :`MyPlayerStatus` "Not Ready" :`Team` (`self.Team Name`))
    (elif (< (`KismetArrayLibrary.Array_Length` (`/Game/BluePrints/Gameplay/PayloadGM.PlayersEngineers` _aspayload_gm)) (+ (`KismetArrayLibrary.Array_Length` (`/Game/BluePrints/Gameplay/PayloadGM.EngineersTeamStart` _aspayload_gm)) 1))
      (`KismetArrayLibrary.Array_Add` (`/Game/BluePrints/Gameplay/PayloadGM.PlayersEngineers` _aspayload_gm) _myplayername)
      (set `self.Team Name` "Engineers")
      (else
        (`GameplayStatics.OpenLevel` "MainMenu")))))

(fn `UserConstructionScript`)