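; PLGS, apparently the game state for a multiplayer test, gates match start on player count and readiness.
; On authority it caches the PLGM game mode and its MaxPlayers at BeginPlay.
; When full, CanStart? loops over player controllers, overwriting GameCanStart each time so the last decides, then shows the countdown or retries after a second.
; Nothing follows the countdown delay, and StartMatch is empty.
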(event `self.ReceiveBeginPlay`
  (`/Engine/EditorBlueprintResources/ActorMacros.Switch Has Authority`
    (:`Authority`
      (bind _asplgm (cast `/Game/BluePrints/Tests/PLGM` (`GameplayStatics.GetGameMode`)))
      (set `self.PLGM REF` _asplgm)
      (set `self.Max Players` (`/Game/BluePrints/Tests/PLGM.Max Players` _asplgm)))))

(event `CanStart?`
  (params (`Current Players` :type Integer))
  (bind _plgm_ref (`self.PLGM REF`))
  (bind _output_get (set `self.Current Players` `Current Players`))
  (if (== _output_get (`self.Max Players`))
    (for _array_element (`/Game/BluePrints/Tests/PLGM.AllPlayerControllers` _plgm_ref)
      (bind _asplpc (cast `/Game/BluePrints/Tests/PLPC` _array_element))
      (if (`/Game/BluePrints/Tests/PLPC.ReadyToStart?` _asplpc)
        (set `self.GameCanStart?` true)
        (else
          (set `self.GameCanStart?` false))))
    (if (`self.GameCanStart?`)
      (`/Game/BluePrints/Tests/PLGM.Show Countdown` _plgm_ref)
      (`KismetSystemLibrary.Delay` 5.0)
      (else
        (`KismetSystemLibrary.PrintString` "Not Ready to start!")
        (`KismetSystemLibrary.Delay` 1.0)
        (`self.CanStart?` (`self.Current Players`))))))

(event `Start Match`)

(fn `UserConstructionScript`)