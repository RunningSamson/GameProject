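; Multiplayer game mode that tracks joining players, starts the match and spawns each player's chosen character on a team start.
; On login it reads server settings from the game instance, sets up the PLPC, sends the rebuilt player list to all controllers and asks PLGS whether play can start.
; ShowCountdown notifies every controller and immediately calls StartMatch.
; PlayerStarts are split by tag at BeginPlay for random team spawns; deaths are forwarded to the PLPC.
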(event `self.ReceiveBeginPlay`
  ;[1 1 1] Get All Spawnpoints
  (bind _outactors (`GameplayStatics.GetAllActorsOfClass` "/Script/Engine.PlayerStart"))
  (set `self.Spawn Points` _outactors)
  (`self.Sort Player Start Point`))

(event `self.K2_PostLogin`
  (params (NewPlayer :type "PlayerController Object Reference"))
  ;[1 1 1] OnPostLogin
  (`/Engine/EditorBlueprintResources/ActorMacros.Switch Has Authority`
    (:`Authority`
      (`KismetArrayLibrary.Array_Add` (`self.AllPlayerControllers`) NewPlayer)
      (bind _asgame_info_instance (cast `/Game/BluePrints/AllLevels/GameInfoInstance` (`GameplayStatics.GetGameInstance`)))
      (set `self.Max Players` (`/Game/BluePrints/AllLevels/GameInfoInstance.MaxPlayers` _asgame_info_instance))
      (set `self.Server Name` (`/Game/BluePrints/AllLevels/GameInfoInstance.Server Name` _asgame_info_instance))
      (set `self.CurrentPlayers` (+ (`self.CurrentPlayers`) 1))
      (bind _asplpc (cast `/Game/BluePrints/Tests/PLPC` NewPlayer))
      (`/Game/BluePrints/Tests/PLPC.Initial Setup` _asplpc)
      (`self.All Update`)
      (bind _asplgs (cast `/Game/BluePrints/Tests/PLGS` (`GameplayStatics.GetGameState`)))
      (`/Game/BluePrints/Tests/PLGS.CanStart?` _asplgs (`self.CurrentPlayers`)))))

(event `All Update`
  (bind _allplayercontrollers (`self.AllPlayerControllers`))
  ;[1 1 1] Update All Players
  (bind _output_get (set `self.CurrentPlayers` (`KismetArrayLibrary.Array_Length` (`self.AllPlayerControllers`))))
  (if (> _output_get 0)
    (`KismetArrayLibrary.Array_Clear` (`self.Connected Players`))
    (for _array_element _allplayercontrollers
      (bind _asplpc (cast `/Game/BluePrints/Tests/PLPC` _array_element))
      (`KismetArrayLibrary.Array_Add` (`self.Connected Players`) (`/Game/BluePrints/Tests/PLPC.PlayerSettings` _asplpc)))
    (for _array_element_2 _allplayercontrollers
      (bind _asplpc_2 (cast `/Game/BluePrints/Tests/PLPC` _array_element_2))
      (`/Game/BluePrints/Tests/PLPC.Add Player Info` _asplpc_2 (`self.Connected Players`)))))

(event `Show Countdown`
  ;[1 1 1] Show Countdown
  (for _array_element (`self.AllPlayerControllers`)
    (bind _asplpc (cast `/Game/BluePrints/Tests/PLPC` _array_element))
    (`/Game/BluePrints/Tests/PLPC.Show Countdown` _asplpc))
  (`self.StartMatch`))

(event `Player Has Died`
  (params (`Player Pawn` :type "Character Object Reference"))
  ;[1 1 1] Player Has Died
  (bind _asplpc (cast `/Game/BluePrints/Tests/PLPC` (`Pawn.GetController` `Player Pawn`)))
  (`/Game/BluePrints/Tests/PLPC.OnDeath` _asplpc))

(event `Spawn For First Time`
  (params (PlayerController :type "PlayerController Object Reference"))
  (bind _playerstart_teama (`self.PlayerStart TeamA`))
  (bind _playerstart_teamb (`self.PlayerStart TeamB`))
  ;[1 1 1] Spawn For The First Time
  (bind _asplpc (cast `/Game/BluePrints/Tests/PLPC` PlayerController))
  (`/Engine/EditorBlueprintResources/StandardMacros.IsValid` (`Controller.K2_GetPawn` PlayerController)
    (:`Is Not Valid`
      (bind (_myplayername _myplayerimg _myplayercharacter _myplayercharacterimg _myplayerstatus _myteamname) (break `/Game/BluePrints/AllLevels/PlayerInfo` (`/Game/BluePrints/Tests/PLPC.PlayerSettings` _asplpc)))
      (if (`KismetStringLibrary.EqualEqual_StrStr` (`KismetTextLibrary.Conv_TextToString` _myteamname) "TeamA")
        (bind _returnvalue (`|SpawnActorFromClass` _myplayercharacter (`self.GetTransform` (`|GetArrayItem` _playerstart_teama (`KismetMathLibrary.RandomIntegerInRange` 0 (- (`KismetArrayLibrary.Array_Length` _playerstart_teama) 1)))) "Undefined" "OverrideRootScale" null null))
        (`KismetSystemLibrary.PrintString` (`KismetSystemLibrary.GetClassDisplayName` _myplayercharacter) true true (struct :`R` 0.983147 :`G` 1.0 :`A` 1.0) 50.0)
        (`KismetSystemLibrary.Delay` 1.0)
        (`Controller.Possess` PlayerController _returnvalue)
        (else
          (bind _returnvalue_2 (`|SpawnActorFromClass` _myplayercharacter (`self.GetTransform` (`|GetArrayItem` _playerstart_teamb (`KismetMathLibrary.RandomIntegerInRange` 0 (- (`KismetArrayLibrary.Array_Length` _playerstart_teamb) 1)))) "Undefined" "OverrideRootScale" null null))
          (`KismetSystemLibrary.PrintString` (`KismetSystemLibrary.GetClassDisplayName` _myplayercharacter) true true (struct :`R` 0.983147 :`G` 1.0 :`A` 1.0) 50.0)
          (`KismetSystemLibrary.Delay` 1.0)
          (`Controller.Possess` PlayerController _returnvalue_2))))))

(fn `Sort Player Start Point`
  (bind _outactors (`GameplayStatics.GetAllActorsOfClass` "/Script/Engine.PlayerStart"))
  (for _array_element _outactors
    (if (`KismetStringLibrary.EqualEqual_StrStr` (`KismetStringLibrary.Conv_NameToString` (`PlayerStart.PlayerStartTag` _array_element)) "TeamA")
      (`KismetArrayLibrary.Array_Add` (`self.PlayerStart TeamA`) _array_element)
      (else
        (`KismetArrayLibrary.Array_Add` (`self.PlayerStart TeamB`) _array_element)))))

(fn `UserConstructionScript`)